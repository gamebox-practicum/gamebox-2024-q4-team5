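; Time beacon actor that visualises a timer through a light and particle column, with start and stop events.
; A timeline curve drives the rect light intensity and the particle system scale, the latter also divided by the set Time.
; Starting plays an attached torch-dying sound, while stopping reverses the timeline.
; An optional TestLight reference receives the same time and mirrors play and reverse.
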(event `self.EventSetTimeForTimer`
  (params (Time :type "Float (single-precision) (by ref)"))
  (bind _output_get (set `self.Time` Time))
  (bind _testlight (`self.TestLight`)
    (:`then`
      (set `/Game/SK/Blueprints/Tools/BP_TestLight.Time` _output_get _testlight))
    (:`else`)))

(event `self.EventPlayTimer`
  (`|ExecutionSequence`
    (:`then_0`
      (`|ExecutionSequence`
        (:`then_0`
          (bind (_direction _newtrack_0) (`Timeline|Timeline: Column lighting` :`NewTime` (`self.Time`) :!via `PlayFromStart` :!label _label)
            (:`Update`
              (`LightComponent.SetIntensity` (`self.RectLight`) (* (`self.MaxIntensity`) _newtrack_0))
              (`SceneComponent.SetRelativeScale3D` (`self.ParticleSystem`) (/ (* (1.0 1.0 1.0) _newtrack_0) (`self.Time`))))))
        (:`then_1`
          (`GameplayStatics.SpawnSoundAttached` "/Game/SK/Assets/Sounds/Sound/event/event_torch_dies.event_torch_dies" (`self.RootComponent`) "None" (0.0 0.0 0.0) (struct) "KeepRelativeOffset" true 1.0 1.0 0.0 "/Game/SK/Assets/Sounds/ATT_DistanceEffect.ATT_DistanceEffect" null))))
    (:`then_1`
      (bind _testlight (`self.TestLight`)
        (:`then`
          (`/Game/SK/Blueprints/Tools/BP_TestLight.Timeline_Play` _testlight))
        (:`else`)))))

(event `self.EventStopTimer`
  (`|ExecutionSequence`
    (:`then_0`
      (goto _label :!via `Reverse`))
    (:`then_1`
      (bind _testlight (`self.TestLight`)
        (:`then`
          (`/Game/SK/Blueprints/Tools/BP_TestLight.Timeline_Reverse` _testlight))
        (:`else`)))))

(fn `UserConstructionScript`)