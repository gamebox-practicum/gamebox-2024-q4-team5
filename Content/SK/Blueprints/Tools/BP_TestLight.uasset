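; BP_TestLight is a point light whose intensity is tied to the stage progression of the chess operator.
; At BeginPlay it stores its maximum intensity, finds the first BP_ChessOperator_Base and switches off if the current stage is below ControlStage.
; A timeline scales intensity by that maximum, with play and reverse events gated on the stage.
; OnNextStage reverses the timeline from its end when ControlStage is reached.
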(event `self.ReceiveBeginPlay`
  (set `self.MaxIntensity` (`LightComponentBase.Intensity` (`self.PointLight`)))
  (bind _outactors (`GameplayStatics.GetAllActorsOfClass` "/Game/SK/Blueprints/ChessOperators/BP_ChessOperator_Base.BP_ChessOperator_Base_C"))
  (bind _output_get (set `self.CurrentOperator` (`|GetArrayItem` _outactors)))
  (`/Engine/EditorBlueprintResources/StandardMacros.IsValid` _output_get
    (:`Is Valid`
      (if (not (>= (`ChessOperator.CurrentStageNum` (`self.CurrentOperator`)) (`self.ControlStage`)))
        (`LightComponent.SetIntensity` (`self.PointLight`) 0.0)))))

(event `Timeline_Play`
  (if (>= (`ChessOperator.CurrentStageNum` (`self.CurrentOperator`)) (`self.ControlStage`))
    (bind (_direction _newtrack_0) (`Timeline|Timeline_0` :`NewTime` (`self.Time`) :!via `PlayFromStart` :!label _label)
      (:`Update`
        (`LightComponent.SetIntensity` (`self.PointLight`) (* _newtrack_0 (`self.MaxIntensity`)))))))

(event `Timeline_Reverse`
  (if (>= (`ChessOperator.CurrentStageNum` (`self.CurrentOperator`)) (`self.ControlStage`))
    (if (!= (`LightComponentBase.Intensity` (`self.PointLight`)) 0.0)
      (goto _label :!via `Reverse`)
      (else
        (goto _label :!via `ReverseFromEnd`)))))

(event `On Next Stage`
  (params (Stage :type Integer))
  (if (== Stage (`self.ControlStage`))
    (goto _label :!via `ReverseFromEnd`)))

(fn `UserConstructionScript`)