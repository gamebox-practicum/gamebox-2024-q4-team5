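; BP_ActorRepeatSound is a utility that plays a sound repeatedly on its owning actor until stopped.
; PlaySound waits a random delay up to RepeatInterval, then spawns the sound attached to the owner's root component with distance attenuation.
; Each audio component's finished event restarts that delay-and-spawn cycle unless IsStopped is set.
; StopSound sets that flag and stops the current audio component.
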(event `PlaySound`
  (`KismetSystemLibrary.Delay` (`KismetMathLibrary.RandomFloatInRange` 0.0 (`self.RepeatInterval`)) :!label _label)
  (bind _returnvalue (`GameplayStatics.SpawnSoundAttached` (`self.Sound`) (`Actor.RootComponent` (`self.GetOwner`)) "None" (0.0 0.0 0.0) (struct) "KeepRelativeOffset" true (`self.Volume Multiplier`) 1.0 0.0 "/Game/SK/Assets/Sounds/ATT_DistanceEffect.ATT_DistanceEffect" null))
  (bind _output_get (set `self.CurrentAudioComponent` _returnvalue))
  (add `AudioComponent.OnAudioFinished` _output_get (delegate `OnSoundFinish`)))

(event `OnSoundFinish`
  (if (not (`self.IsStopped?`))
    (goto _label)))

(event `StopSound`
  (set `self.IsStopped?` true)
  (bind _currentaudiocomponent (`self.CurrentAudioComponent`)
    (:`then`
      (`AudioComponent.Stop` _currentaudiocomponent))
    (:`else`)))