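; Game mode for the main menu level that sets up the menu UI when play begins.
; On BeginPlay it casts the first player controller to BP_PlayerController_MainMenu, switches it to UI-only input and shows the mouse cursor.
; It creates WBP_MainMenu, stores it on that controller, adds it to the viewport and plays a 2D sound.
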(event `self.ReceiveBeginPlay`
  (`parent.ReceiveBeginPlay`)
  (bind _asbp_player_controller_main_menu (cast `/Game/SK/Blueprints/Core/Menu/BP_PlayerController_MainMenu` (`GameplayStatics.GetPlayerController` 0)))
  (`WidgetBlueprintLibrary.SetInputMode_UIOnlyEx` _asbp_player_controller_main_menu null)
  (bind _returnvalue (`|CreateWidget` "/Game/SK/Blueprints/Widgets/Menu/WBP_MainMenu.WBP_MainMenu_C" _asbp_player_controller_main_menu))
  (bind _output_get (set `/Game/SK/Blueprints/Core/Menu/BP_PlayerController_MainMenu.Current WBP Main Menu` _returnvalue _asbp_player_controller_main_menu))
  (`UserWidget.AddToViewport` _output_get 0)
  (set `PlayerController.bShowMouseCursor` true _asbp_player_controller_main_menu)
  (`GameplayStatics.PlaySound2D` null 1.0 1.0 0.0 null null))

(fn `UserConstructionScript`
  (`parent.UserConstructionScript`))