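; Player controller that owns the pause menu and handles losing and finishing the game.
; SetPause switches widget visibility, input mode, cursor and game pause, clearing note scene widgets on unpause.
; Losing shows a UI-only lose window, while finishing stores the good-ending flag in the GameInstance from the collected note count.
; The ending plays a fade sequence in reverse with a stop callback, and Play_End advances the GameInstance to the next level.
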(event `self.ReceiveBeginPlay`
  (bind _returnvalue (`|CreateWidget` "/Game/LawnMoverGame/Blueprints/UI/Menu/W_Pause.W_Pause_C" self))
  (bind _output_get (set `self.PauseWindow` _returnvalue))
  (`self.SetPause` false)
  (`UserWidget.AddToViewport` _output_get 0))

(event `InputAction|Paused` :paused true
  (params (Key :type "Key Structure"))
  (:`Pressed`
    (`/Game/LawnMoverGame/Blueprints/UI/Menu/W_Pause.OnPauseAction` (`self.PauseWindow`))))

(event `Play_End`
  (bind _asbp_game_instance (cast `/Game/SK/Blueprints/Core/BP_GameInstance` (`GameplayStatics.GetGameInstance`)))
  (`SK_GameInstance.NextLevel` _asbp_game_instance))

(fn `OnGameEnd`
  (set `self.IsGameOver` true)
  (bind _asbp_game_mode (cast `/Game/SK/Blueprints/Core/Game/BP_GameMode` (`GameplayStatics.GetGameMode`)))
  (bind _asbp_game_instance (cast `/Game/SK/Blueprints/Core/BP_GameInstance` (`GameplayStatics.GetGameInstance`)))
  (set `SK_GameInstance.bIsGoodEnd` (<= (`self.WinNotesCount`) (`KismetArrayLibrary.Array_Length` (`/Game/SK/Blueprints/Core/Game/BP_GameMode.CollectedNotes` _asbp_game_mode))) _asbp_game_instance)
  (bind (_outactor _returnvalue) (`LevelSequencePlayer.CreateLevelSequencePlayer` "/Game/SK/Maps/LS_FadeTrack.LS_FadeTrack"))
  (`MovieSceneSequencePlayer.PlayReverse` _returnvalue)
  (add `MovieSceneSequencePlayer.OnStop` _returnvalue (`|CreateDelegate` :!event `Play_End`)))

(fn `OnGameLoose`
  (set `self.IsGameOver` true)
  (bind _returnvalue (`|CreateWidget` "/Game/SK/Blueprints/UI/WBP_LoseGameWindow.WBP_LoseGameWindow_C"))
  (`UserWidget.AddToViewport` _returnvalue 0)
  (`WidgetBlueprintLibrary.SetInputMode_UIOnlyEx` self null)
  (set `PlayerController.bShowMouseCursor` true))

(fn `SetPause`
  (params (value :type Boolean))
  (if value
    (set `self.IsPaused` true)
    (`Widget.SetVisibility` (`self.PauseWindow`) "Visible")
    (`WidgetBlueprintLibrary.SetInputMode_GameAndUIEx` self null "DoNotLock" false)
    (set `PlayerController.bShowMouseCursor` true)
    (`GameplayStatics.SetGamePaused` true)
    (else
      (set `self.IsPaused` false)
      (`Widget.SetVisibility` (`self.PauseWindow`) "Hidden")
      (`WidgetBlueprintLibrary.SetInputMode_GameOnly` self)
      (set `PlayerController.bShowMouseCursor` false)
      (`GameplayStatics.SetGamePaused` false)
      (bind _foundwidgets (`WidgetBlueprintLibrary.GetAllWidgetsOfClass` "/Game/SK/Blueprints/UI/WBP_Note_scene.WBP_Note_scene_C"))
      (for _array_element _foundwidgets
        (`Widget.RemoveFromParent` _array_element)))))

(fn `TogglePause`
  (`self.SetPause` (not (`self.IsPaused`))))

(fn `UserConstructionScript`)