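; Game mode that handles level start, win and lose outcomes, and pausing on window focus loss.
; On BeginPlay it caches BP_GameInstance, plays start and ambient sounds, and runs a fade level sequence.
; Win and lose events notify every BP_PlayerController, while focus loss pauses through player controller 0.
; ShowBloodMonitor adds the blood overlay widget only if the saved settings enable blood.
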(event `self.ReceiveBeginPlay`
  (`|ExecutionSequence`
    (:`then_0`
      (bind _asbp_game_instance (cast `/Game/SK/Blueprints/Core/BP_GameInstance` (`GameplayStatics.GetGameInstance`)))
      (set `self.CurrentGameInstance` _asbp_game_instance))
    (:`then_1`
      (`GameplayStatics.PlaySound2D` "/Game/SK/Assets/Sounds/Events/A_Event_Game_Start.A_Event_Game_Start" 1.0 1.0 0.0 null null)
      (`GameplayStatics.PlaySound2D` "/Game/SK/Assets/Sounds/Loop/A_Loop_Ambient_v1.A_Loop_Ambient_v1" 1.0 1.0 0.0 null null))
    (:`then_2`
      (bind (_outactor _returnvalue) (`LevelSequencePlayer.CreateLevelSequencePlayer` "/Game/SK/Maps/LS_FadeTrack.LS_FadeTrack"))
      (`MovieSceneSequencePlayer.Play` _returnvalue))))

(event `self.EventLosingGame`
  (bind _outactors (`GameplayStatics.GetAllActorsOfClass` "/Game/SK/Blueprints/Core/Game/BP_PlayerController.BP_PlayerController_C"))
  (for _array_element _outactors
    (`/Game/SK/Blueprints/Core/Game/BP_PlayerController.OnGameLoose` _array_element)))

(event `self.EventWinningGame`
  (bind _outactors (`GameplayStatics.GetAllActorsOfClass` "/Game/SK/Blueprints/Core/Game/BP_PlayerController.BP_PlayerController_C"))
  (for _array_element _outactors
    (`/Game/SK/Blueprints/Core/Game/BP_PlayerController.OnGameEnd` _array_element)))

(event `self.OnWindowsLostFocus`
  (bind _asbp_player_controller (cast `/Game/SK/Blueprints/Core/Game/BP_PlayerController` (`GameplayStatics.GetPlayerController` 0)))
  (`/Game/SK/Blueprints/Core/Game/BP_PlayerController.SetPause` _asbp_player_controller true))

(fn `ShowBloodMonitor`
  (if (`.bBloodIsShown` (break `SettingsData` (`SaveSettings.SettingsData` (`SK_GameInstance.SaveSettings` (`self.CurrentGameInstance`)))))
    (bind _returnvalue (`|CreateWidget` "/Game/SK/Blueprints/Widgets/Game/WBP_BloodMonitor.WBP_BloodMonitor_C"))
    (`UserWidget.AddToViewport` _returnvalue 0)))

(fn `UserConstructionScript`)