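; Test Blueprint that runs the chess AI against itself on BeginPlay.
; It constructs an 8x8 ChessBoardInfo with only a white and a black King in opposite corners.
; A fixed-length loop asks GetNextStep for a depth-limited move for White, then Black, applying each with DoStep and logging the board.
; Black moves only if White could, and an unable move does not end the loop.
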(event `self.ReceiveBeginPlay`
  (bind _newvar_0 (`self.NewVar_0`))
  (bind _returnvalue (`|GenericCreateObject` "/Script/SK.ChessBoardInfo" self))
  (bind _output_get (set `self.NewVar_0` _returnvalue))
  (`ChessBoardInfo.Init` _output_get 8 8)
  (`|ExecutionSequence`
    (:`then_0`
      (bind _returnvalue_2 (`|GenericCreateObject` "/Script/SK.King" self))
      (set `ChessPieceInfo.Color` "WHITE" _returnvalue_2)
      (`ChessBoardInfo.Set` (`self.NewVar_0`) 0 0 _returnvalue_2))
    (:`then_1`
      (bind _returnvalue_3 (`|GenericCreateObject` "/Script/SK.King" self))
      (set `ChessPieceInfo.Color` "BLACK" _returnvalue_3)
      (`ChessBoardInfo.Set` (`self.NewVar_0`) 7 7 _returnvalue_3))
    (:`then_2`
      (`ChessAILibrary.LogChessBoard` (`self.NewVar_0`)))
    (:`then_3`
      (for _index (range 21)
        (`KismetSystemLibrary.PrintString` (`KismetStringLibrary.Conv_IntToString` _index))
        (bind _returnvalue_4 (`ChessAILibrary.GetNextStep` (`self.NewVar_0`) "WHITE" 4))
        (if (not (`ChessAILibrary.IsUnableMove` _returnvalue_4))
          (`ChessAILibrary.DoStep` _returnvalue_4 (`self.NewVar_0`))
          (`ChessAILibrary.LogChessBoard` _newvar_0)
          (bind _returnvalue_5 (`ChessAILibrary.GetNextStep` _newvar_0 "BLACK" 4))
          (if (not (`ChessAILibrary.IsUnableMove` _returnvalue_5))
            (`ChessAILibrary.DoStep` _returnvalue_5 (`self.NewVar_0`))
            (`ChessAILibrary.LogChessBoard` (`self.NewVar_0`))))))))

(fn `UserConstructionScript`)